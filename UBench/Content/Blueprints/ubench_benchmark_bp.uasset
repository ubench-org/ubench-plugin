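; Benchmark actor that measures frame rate over a timed run and reports results in an overlay widget it creates.
; Starts on BeginPlay or in manual mode with a cursor, warms up briefly and can apply engine hardware benchmark settings.
; Tick samples FPS while timers drive progress and the automatic stop.
; The report shows min, max, average, a threshold-based score and a sample graph, with dispatchers marking each start and stop phase.
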(event `self.ReceiveBeginPlay`
  (bind _returnvalue (`GameplayStatics.GetPlayerController` 0))
  (bind _manual_start (`self.Manual Start`))
  (`|ExecutionSequence`
    (:`then_0`
      (bind _returnvalue_2 (`|CreateWidget` "/UBench/UI/ubench_overlay_uI.ubench_overlay_ui_C" null self _manual_start))
      (bind _output_get (set `self.ubench overlay ui reference` _returnvalue_2))
      (`UserWidget.AddToViewport` _output_get 999999999))
    (:`then_1`
      (if _manual_start
        (`WidgetBlueprintLibrary.SetInputMode_GameAndUIEx` _returnvalue _output_get "LockAlways" false)
        (set `PlayerController.bShowMouseCursor` true _returnvalue)
        (else
          (`self.Start Benchmarking`))))))

(event `Start Benchmarking`
  (bind _ubench_overlay_ui_reference (`self.ubench overlay ui reference`))
  (bind _btn_start_stop (`/UBench/UI/ubench_overlay_uI.btn_start_stop` _ubench_overlay_ui_reference))
  (bind _txt_status (`/UBench/UI/ubench_overlay_uI.txt_status` _ubench_overlay_ui_reference))
  (if (not (`self.benchmarking`))
    (`self.Benchmark Starting`)
    (`self.Reset Counters`)
    (`ProgressBar.SetIsMarquee` (`/UBench/UI/ubench_overlay_uI.prg_progress` (`self.ubench overlay ui reference`)) true)
    (`TextBlock.SetText` _txt_status "Warming Up...")
    (`KismetSystemLibrary.Delay` 1.0)
    (`TextBlock.SetText` _txt_status (`|FormatText` "Running {difficulty}" (`|GetEnumeratorNameAsString` (`self.Difficulty`))))
    (`|ExecutionSequence`
      (:`then_0`
        (if (`self.Run Hardware Benchmark`)
          (bind _returnvalue (`GameUserSettings.GetGameUserSettings`))
          (`GameUserSettings.RunHardwareBenchmark` _returnvalue 10 1.0 1.0)
          (`GameUserSettings.ApplyHardwareBenchmarkResults` _returnvalue))
        (set `self.benchmarking` true)
        (`self.Benchmark Started`))
      (:`then_1`
        (`Widget.SetVisibility` (`/UBench/UI/ubench_overlay_uI.box_results` _ubench_overlay_ui_reference) "Collapsed"))
      (:`then_2`
        (`Button.SetBackgroundColor` _btn_start_stop (struct :`R` 0.300544 :`A` 1.0))
        (`TextBlock.SetText` (`/UBench/UI/ubench_overlay_uI.txt_start_stop` _ubench_overlay_ui_reference) "Stop")
        (`Widget.SetIsEnabled` _btn_start_stop true))
      (:`then_3`
        (`KismetSystemLibrary.K2_SetTimerDelegate` (delegate `Stop Benchmarking`) (`self.Duration`))
        (bind _returnvalue_2 (`KismetSystemLibrary.K2_SetTimerDelegate` (delegate `Tick Progress`) 0.1 true))
        (set `self.tick progress timer` _returnvalue_2)))))

(event `Reset Counters`
  (`|ExecutionSequence`
    (:`then_0`
      (set `self.FPS` 0.0))
    (:`then_1`
      (set `self.FPS Min` 999.0))
    (:`then_2`
      (set `self.FPS Max` -1.0))
    (:`then_3`
      (set `self.Delta Seconds` 0.0))
    (:`then_4`
      (set `self.FPS Avg` 0.0))
    (:`then_5`
      (set `self.Last FPS` 0.0))
    (:`then_6`
      (`KismetArrayLibrary.Array_Clear` (`self.samples`)))
    (:`then_7`
      (set `self.Progress` 0.0))
    (:`then_8`
      (set `self.samples sum` 0.0))))

(event `Tick Progress`
  (bind _prg_progress (`/UBench/UI/ubench_overlay_uI.prg_progress` (`self.ubench overlay ui reference`)))
  (`|ExecutionSequence`
    (:`then_0`
      (`/Engine/EditorBlueprintResources/StandardMacros.DoOnce` false
        (:`Completed`
          (`ProgressBar.SetIsMarquee` _prg_progress false))))
    (:`then_1`
      (set `self.Progress` (+ (`self.Progress`) 0.1)))
    (:`then_2`
      (`ProgressBar.SetPercent` _prg_progress (/ (`self.Progress`) (`self.Duration`))))))

(event `Stop Benchmarking`
  (bind _ubench_overlay_ui_reference (`self.ubench overlay ui reference`))
  (bind _btn_start_stop (`/UBench/UI/ubench_overlay_uI.btn_start_stop` _ubench_overlay_ui_reference))
  (if (`self.benchmarking`)
    (`self.Benchmark Stopping`)
    (`|ExecutionSequence`
      (:`then_0`
        (set `self.benchmarking` false))
      (:`then_1`
        (`KismetSystemLibrary.K2_PauseTimerHandle` (`self.tick progress timer`)))
      (:`then_2`
        (`MeshComponent.SetVectorParameterValueOnMaterials` (`self.ubench_logo_ring_sm`) "color" (`KismetMathLibrary.Conv_LinearColorToVector` (struct :`R` 1.0 :`G` 1.0 :`B` 1.0 :`A` 1.0))))
      (:`then_3`
        (`Button.SetBackgroundColor` _btn_start_stop (struct :`R` 0.019382 :`G` 0.300544 :`A` 1.0))
        (`TextBlock.SetText` (`/UBench/UI/ubench_overlay_uI.txt_start_stop` _ubench_overlay_ui_reference) "Start")
        (`Widget.SetIsEnabled` _btn_start_stop true))
      (:`then_4`
        (`TextBlock.SetText` (`/UBench/UI/ubench_overlay_uI.txt_status` _ubench_overlay_ui_reference) "Stopped"))
      (:`then_6`
        (`self.Generate Report`))
      (:`then_7`
        (`self.Benchmark Stopped`)))))

(event `self.ReceiveTick`
  (params (DeltaSeconds :type "Float (single-precision)"))
  (bind _fps (`self.FPS`))
  (set `self.Delta Seconds` DeltaSeconds)
  (if (`self.benchmarking`)
    (bind _output_get (set `self.FPS` (/ 1.0 (`self.Delta Seconds`))))
    (`KismetArrayLibrary.Array_Add` (`self.samples`) _output_get)
    (`|ExecutionSequence`
      (:`then_0`
        (if (< _output_get (`self.FPS Min`))
          (set `self.FPS Min` _fps)))
      (:`then_1`
        (if (> _output_get (`self.FPS Max`))
          (set `self.FPS Max` _fps))))))

(event `Generate Report`
  (bind _ubench_overlay_ui_reference (`self.ubench overlay ui reference`))
  (bind _value_precision (`self.Value Precision`))
  (`|ExecutionSequence`
    (:`then_2`
      (`TextBlock.SetText` (`/UBench/UI/ubench_overlay_uI.txt_fps_min` _ubench_overlay_ui_reference) (`KismetTextLibrary.Conv_DoubleToText` (`self.FPS Min`) "HalfToEven" false true 1 324 _value_precision _value_precision))
      (`TextBlock.SetText` (`/UBench/UI/ubench_overlay_uI.txt_fps_max` _ubench_overlay_ui_reference) (`KismetTextLibrary.Conv_DoubleToText` (`self.FPS Max`) "HalfToEven" false true 1 324 _value_precision _value_precision))
      (bind _output_get (`self.Calculate Average FPS`))
      (`TextBlock.SetText` (`/UBench/UI/ubench_overlay_uI.txt_fps_avg` _ubench_overlay_ui_reference) (`KismetTextLibrary.Conv_DoubleToText` _output_get "HalfToEven" false true 1 324 _value_precision _value_precision)))
    (:`then_3`
      (`TextBlock.SetText` (`/UBench/UI/ubench_overlay_uI.txt_score` _ubench_overlay_ui_reference) (`KismetTextLibrary.Conv_StringToText` (`|GetEnumeratorNameAsString` (`self.To Score`)))))
    (:`then_4`
      (`Widget.SetVisibility` (`/UBench/UI/ubench_overlay_uI.box_results` _ubench_overlay_ui_reference) "Visible"))
    (:`then_5`
      (`/UBench/UI/ubench_report_graph_ui.Build Graph` (`/UBench/UI/ubench_overlay_uI.ubench_report_graph_ui` (`self.ubench overlay ui reference`)) (`self.samples`)))))

(fn `Calculate Average FPS`
  (returns (Output_Get :type "Float (double-precision)"))
  (bind _samples (`self.samples`))
  (set `self.samples sum` 0.0)
  (for _array_element _samples
    (set `self.samples sum` (+ (`self.samples sum`) _array_element)))
  (bind _output_get (set `self.FPS Avg` (/ (`self.samples sum`) (`KismetMathLibrary.Conv_IntToDouble` (`KismetArrayLibrary.Array_Length` _samples)))))
  (return _output_get))

(fn `To Score`
  (returns (Score :type "/UBench/Data/scores_enum Enum"))
  (locals (_score :type "/UBench/Data/scores_enum Enum") (`score byte` :type "/UBench/Data/scores_enum Enum"))
  (bind _output_get (`self.Calculate Average FPS`))
  (`KismetSystemLibrary.PrintString` (`KismetStringLibrary.Conv_DoubleToString` _output_get) true true (struct :`G` 0.66 :`B` 1.0 :`A` 1.0) 5.0)
  (`|ExecutionSequence`
    (:`then_0`
      (if (< _output_get 10.0)
        (set `local._score` "NewEnumerator0")
        (elif (`KismetMathLibrary.InRange_FloatFloat` _output_get 0.0 15.0 false)
          (set `local._score` "NewEnumerator1")
          (elif (`KismetMathLibrary.InRange_FloatFloat` _output_get 15.0 45.0 false)
            (set `local._score` "NewEnumerator2")
            (elif (`KismetMathLibrary.InRange_FloatFloat` _output_get 45.0 60.0 false)
              (set `local._score` "NewEnumerator3")
              (elif (`KismetMathLibrary.InRange_FloatFloat` _output_get 60.0 120.0 false)
                (set `local._score` "NewEnumerator4")
                (elif (> _output_get 120.0)
                  (set `local._score` "NewEnumerator5"))))))))
    (:`then_6`
      (return (`local._score`)))))

(fn `UserConstructionScript`
  (`self.SetActorTickInterval` 0.0))